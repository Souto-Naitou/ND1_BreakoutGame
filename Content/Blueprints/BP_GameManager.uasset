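; Game manager for a Breakout-style level that tracks blocks and remaining balls and decides clear and game over.
; Block counters trigger the clear widget when none remain, while a miss with no balls left shows game over.
; Action spawns a ball at a marker actor, reloads the level after game over, or opens the next level after a clear.
; BreakoutGameInstance carries the ball count between levels, plus one on clear.
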(event `self.ReceiveBeginPlay`
  (bind _asbreakout_game_instance (cast `/Game/Blueprints/BreakoutGameInstance` (`GameplayStatics.GetGameInstance`)))
  (bind _isvalidballnum (`/Game/Blueprints/BreakoutGameInstance.IsValidBallNum` _asbreakout_game_instance))
  (if _isvalidballnum
    (set `self.LeftBallNum` (`/Game/Blueprints/BreakoutGameInstance.LeftBallNum` _asbreakout_game_instance))))

(fn `Action`
  (if (`self.IsGameOver`)
    (`self.LevelReset`)
    (elif (`self.isCleared`)
      (`self.OpenNextLevel`)
      (else
        (`self.SpawnBall`)))))

(fn `AddBlockNum`
  (bind _result (`/Engine/EditorBlueprintResources/StandardMacros.IncrementInt` (`self.BlockNum`))
    (:`  `
      (`KismetSystemLibrary.PrintString` (`KismetStringLibrary.Concat_StrStr` "AddBlockNum : " (`KismetStringLibrary.Conv_IntToString` _result))))))

(fn `AddBrokenBlockNum`
  (bind _result (`/Engine/EditorBlueprintResources/StandardMacros.IncrementInt` (`self.BlockenBlockNum`))
    (:`  `
      (`KismetSystemLibrary.PrintString` (`KismetStringLibrary.Concat_StrStr` "BrokenBlockNum : " (`KismetStringLibrary.Conv_IntToString` _result)) true true (struct :`G` 0.049957 :`B` 0.33913 :`A` 1.0))
      (bind _leftblocknum (`self.GetLeftBlockNum`))
      (`KismetSystemLibrary.PrintString` (`KismetStringLibrary.Concat_StrStr` "LeftBlockNum : " (`KismetStringLibrary.Conv_IntToString` _leftblocknum)) true true (struct :`R` 0.416684 :`G` 0.148556 :`B` 1.0 :`A` 1.0))
      (bind _leftblocknum_2 (`self.GetLeftBlockNum`))
      (if (== _leftblocknum_2 0)
        (`self.ViewClearWidget`)
        (set `self.isCleared` true)))))

(fn `GetLeftBallNum`
  (returns (LeftBallNum :type Integer))
  (return (`self.LeftBallNum`)))

(fn `GetLeftBlockNum`
  (returns (LeftBlockNum :type Integer))
  (return (- (`self.BlockNum`) (`self.BlockenBlockNum`))))

(fn `LevelReset`
  (bind _returnvalue (`GameplayStatics.GetCurrentLevelName` true))
  (`GameplayStatics.OpenLevel` (`KismetStringLibrary.Conv_StringToName` _returnvalue)))

(fn `MissCount`
  (set `self.IsBallSpawned` false)
  (if (and (<= (`self.LeftBallNum`) 0) (not (`self.isCleared`)))
    (`self.ViewGameOverWidget`)
    (set `self.IsGameOver` true)))

(fn `OpenNextLevel`
  (bind _asbreakout_game_instance (cast `/Game/Blueprints/BreakoutGameInstance` (`GameplayStatics.GetGameInstance`)))
  (set `/Game/Blueprints/BreakoutGameInstance.LeftBallNum` (+ (`self.LeftBallNum`) 1) _asbreakout_game_instance)
  (`GameplayStatics.OpenLevel` (`self.NextLevelName`)))

(fn `SpawnBall`
  (if (and (> (`self.LeftBallNum`) 0) (not (`self.IsBallSpawned`)))
    (`|SpawnActorFromClass` "/Game/Blueprints/BP_Ball.BP_Ball_C" (`KismetMathLibrary.MakeTransform` (`self.K2_GetActorLocation` (`self.SpawnLocationActor`))) "Undefined" "MultiplyWithRoot" null null)
    (set `self.IsBallSpawned` true)
    (bind _result (`/Engine/EditorBlueprintResources/StandardMacros.DecrementInt` (`self.LeftBallNum`))
      (:`  `
        (set `self.LeftBallNum` _result)))))

(fn `UserConstructionScript`)

(fn `ViewClearWidget`
  (bind _returnvalue (`|CreateWidget` "/Game/Blueprints/WBP_ClearWidget.WBP_ClearWidget_C"))
  (`UserWidget.AddToViewport` _returnvalue 0))

(fn `ViewGameOverWidget`
  (bind _returnvalue (`|CreateWidget` "/Game/Blueprints/WBP_GameOverWidget.WBP_GameOverWidget_C"))
  (`UserWidget.AddToViewport` _returnvalue 0))